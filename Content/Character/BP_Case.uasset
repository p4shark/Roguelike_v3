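; BP_Case is an actor for a case with Up and Down parts that reacts to cursor hover.
; Hovering either part enables custom depth on both, likely for an outline, and plays a timeline that rotates the W component in world-space roll.
; When the cursor leaves either part, custom depth turns off and the timeline reverses the rotation.
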(event `self.Down.OnBeginCursorOver`
  (params (TouchedComponent :type "PrimitiveComponent Object Reference"))
  (`PrimitiveComponent.SetRenderCustomDepth` (`self.Down`) true :!label _label)
  (`PrimitiveComponent.SetRenderCustomDepth` (`self.Up`) true)
  (bind (_direction _newtrack_1) (`Timeline|Timeline` :!label _label_2)
    (:`Update`
      (`SceneComponent.K2_SetWorldRotation` (`self.w`) (`KismetMathLibrary.MakeRotator` _newtrack_1) false false))))

(event `self.Up.OnBeginCursorOver`
  (params (TouchedComponent :type "PrimitiveComponent Object Reference"))
  (goto _label))

(event `self.Up.OnEndCursorOver`
  (params (TouchedComponent :type "PrimitiveComponent Object Reference"))
  (`PrimitiveComponent.SetRenderCustomDepth` (`self.Down`) false :!label _label_3)
  (`PrimitiveComponent.SetRenderCustomDepth` (`self.Up`) false)
  (goto _label_2 :!via `Reverse`))

(event `self.Down.OnEndCursorOver`
  (params (TouchedComponent :type "PrimitiveComponent Object Reference"))
  (goto _label_3))

(fn `UserConstructionScript`)